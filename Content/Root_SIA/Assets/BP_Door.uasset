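; BP_Door is a swinging door that opens only when the player holds both keycard A and keycard B.
; A trigger overlap by the player character checks both keycard flags on the game instance.
; With both, a sped-up timeline rotates the door pivot 90 degrees; otherwise, a text render is shown.
; Leaving the trigger hides the text and reverses the timeline to close the door.
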(event `self.Trigger.OnComponentBeginOverlap`
  (params (OverlappedComponent :type "PrimitiveComponent Object Reference") (OtherActor :type "Actor Object Reference") (OtherComp :type "PrimitiveComponent Object Reference") (OtherBodyIndex :type Integer) (bFromSweep :type Boolean) (SweepResult :type "HitResult Structure (by ref)"))
  (cast `/Game/Root_SIA/Core/Framework/Core_PlayerCharacter` OtherActor)
  (bind _ascore_game_instance (cast `/Game/Root_SIA/Core/Framework/Core_GameInstance` (`GameplayStatics.GetGameInstance`)))
  (if (`/Game/Root_SIA/Core/Framework/Core_GameInstance.bHasKeycardA` _ascore_game_instance)
    (if (`/Game/Root_SIA/Core/Framework/Core_GameInstance.bHasKeycardB` _ascore_game_instance)
      (`TimelineComponent.SetPlayRate` (`self.Timeline_0`) 2.0)
      (bind (_direction _rotation) (`Timeline|Timeline_0` :!label _label)
        (:`Update`
          (`SceneComponent.K2_SetRelativeRotation` (`self.DoorPivot`) (`KismetMathLibrary.RLerp` (struct) (struct :`Yaw` 90.0) _rotation) false false)))
      (else
        (`SceneComponent.SetHiddenInGame` (`self.TextRender`) false false :!label _label_2)))
    (else
      (goto _label_2))))

(event `self.Trigger.OnComponentEndOverlap`
  (params (OverlappedComponent :type "PrimitiveComponent Object Reference") (OtherActor :type "Actor Object Reference") (OtherComp :type "PrimitiveComponent Object Reference") (OtherBodyIndex :type Integer))
  (cast `/Game/Root_SIA/Core/Framework/Core_PlayerCharacter` OtherActor)
  (`SceneComponent.SetHiddenInGame` (`self.TextRender`) true false)
  (goto _label :!via `Reverse`))

(fn `UserConstructionScript`)