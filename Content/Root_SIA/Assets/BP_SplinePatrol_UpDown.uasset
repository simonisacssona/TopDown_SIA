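; Patrolling enemy actor that moves a sprite along a spline and visually flags when the player enters its detection trigger.
; Tick advances the distance along the spline at constant speed, sets the sprite's relative location from it, and wraps to the start at the end.
; Trigger overlaps with Core_PlayerCharacter recolor the spotlight between alert and idle colors and print debug messages, with no further reaction.
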(event `self.ReceiveTick`
  (params (DeltaSeconds :type "Float (single-precision)"))
  (bind _currentdistancealongspline (`self.CurrentDistanceAlongSpline`))
  (bind _returnvalue (`SplineComponent.GetSplineLength` (`self.Spline`)))
  ;[1 1 1] Rotating on Spline
  (if (>= _currentdistancealongspline _returnvalue)
    (set `self.CurrentDistanceAlongSpline` 0.0)
    (else
      (bind _output_get (set `self.CurrentDistanceAlongSpline` (`KismetMathLibrary.FInterpTo_Constant` _currentdistancealongspline _returnvalue DeltaSeconds 300.0)))
      (`SceneComponent.K2_SetRelativeLocation` (`self.EnemySprite`) (`SplineComponent.GetLocationAtDistanceAlongSpline` (`self.Spline`) _output_get "Local") false false))))

(event `self.Trigger.OnComponentBeginOverlap`
  (params (OverlappedComponent :type "PrimitiveComponent Object Reference") (OtherActor :type "Actor Object Reference") (OtherComp :type "PrimitiveComponent Object Reference") (OtherBodyIndex :type Integer) (bFromSweep :type Boolean) (SweepResult :type "HitResult Structure (by ref)"))
  ;[1 1 1] Identifying player
  (cast `/Game/Root_SIA/Core/Framework/Core_PlayerCharacter` OtherActor)
  (`KismetSystemLibrary.PrintString` "Detected" true true (struct :`R` 1.0 :`B` 0.009094 :`A` 1.0))
  (`LightComponent.SetLightColor` (`self.SpotLight`) (struct :`R` 1.0 :`G` 0.008526 :`A` 1.0) true))

(event `self.Trigger.OnComponentEndOverlap`
  (params (OverlappedComponent :type "PrimitiveComponent Object Reference") (OtherActor :type "Actor Object Reference") (OtherComp :type "PrimitiveComponent Object Reference") (OtherBodyIndex :type Integer))
  ;[1 1 1] Identifying player
  (cast `/Game/Root_SIA/Core/Framework/Core_PlayerCharacter` OtherActor)
  (`KismetSystemLibrary.PrintString` "lmao where he go" true true (struct :`G` 0.231278 :`B` 1.0 :`A` 1.0))
  (`LightComponent.SetLightColor` (`self.SpotLight`) (struct :`R` 1.0 :`G` 0.658848 :`A` 1.0) true))

(fn `UserConstructionScript`)